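; Rhythm manager Blueprint that plays music and keeps a repeating beat clock.
; On BeginPlay it starts MusicAudio with a start time of 60 / BPM and sets a looping timer at BeatInterval, which is not computed in the graphs.
; Each TriggerBeat call records the game time in LastBeatTime, clears HasPressedThisBeat and prints a debug message; no input check happens here.
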(event `self.ReceiveBeginPlay`
  (`AudioComponent.Play` (`self.MusicAudio`) (/ 60.0 (`self.BPM`)))
  (`KismetSystemLibrary.K2_SetTimer` null "TriggerBeat" (`self.BeatInterval`) true))

(fn `TriggerBeat`
  (set `self.LastBeatTime` (`KismetSystemLibrary.GetGameTimeInSeconds`))
  (set `self.HasPressedThisBeat` false)
  (`KismetSystemLibrary.PrintString` "Beet!"))

(fn `UserConstructionScript`)